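; BP_Bullet is a bullet projectile that damages enemies and penalizes the player for hitting customers.
; It plays a sound at its location on BeginPlay and destroys itself on any hit.
; Hit branches on actor tags: Enemy receives damage attributed to the bullet's owner, while Customer deducts one Money from Player_TP, if above zero.
; A disconnected branch that would add money never runs.
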(event EventBeginPlay
  (Audio|PlaySoundatLocation 0 (Transformation|GetActorLocation) "0, 0, 0" 1.0 1.0 0.0 0 0 0 0))

(event Collision|EventHit
  (params (MyComp :type Primitive%20Component%20Object%20Reference) (Other :type Actor%20Object%20Reference) (OtherComp :type Primitive%20Component%20Object%20Reference) (bSelfMoved :type Boolean) (HitLocation :type Vector :default "0, 0, 0") (HitNormal :type Vector :default "0, 0, 0") (NormalImpulse :type Vector :default "0, 0, 0") (Hit :type Hit%20Result%20Structure%20%28by%20ref%29))
  (if (Actor|ActorHasTag Other "Enemy")
    (Game|Damage|ApplyDamage Other (Variables|Default|GetDamage) 0 (Components|GetOwner) "/Script/Engine.DamageType")
    (Actor|DestroyActor)
    (elif (Actor|ActorHasTag Other "Customer")
      (Actor|DestroyActor)
      (bind _asplayer_tp (Utilities|Casting|CastToPlayer_TP (Game|GetPlayerCharacter 0)))
      (if (> (Variables|/Game/Character/Main_Character/Player_TP.Player_TP_C|GetMoney _asplayer_tp) 0)
        (Variables|/Game/Character/Main_Character/Player_TP.Player_TP_C|SetMoney _asplayer_tp (- (Variables|/Game/Character/Main_Character/Player_TP.Player_TP_C|GetMoney _asplayer_tp) 1)))
      (else
        (Actor|DestroyActor)))))

(fn ConstructionScript)