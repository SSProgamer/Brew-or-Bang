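; BP_EnemyBullet_Beer is an enemy projectile that damages the player and plays a sound when it spawns.
; On hit it takes one Health from a Player-tagged Player_TP and opens the Gameover level at zero or below, otherwise destroying itself.
; Hits on anything else also destroy it.
; Its mesh overlap destroys any overlapping actor, and destroys the bullet too only when that actor is tagged Beer.
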(event OnComponentBeginOverlap(StaticMesh)
  (params (OverlappedComponent :type Primitive%20Component%20Object%20Reference) (OtherActor :type Actor%20Object%20Reference) (OtherComp :type Primitive%20Component%20Object%20Reference) (OtherBodyIndex :type Integer) (bFromSweep :type Boolean) (SweepResult :type Hit%20Result%20Structure%20%28by%20ref%29))
  (if (Actor|ActorHasTag OtherActor "Beer")
    (Actor|DestroyActor OtherActor)
    (Actor|DestroyActor)
    (else
      (Actor|DestroyActor OtherActor))))

(event EventBeginPlay
  (Audio|PlaySoundatLocation 0 (Transformation|GetActorLocation) "0, 0, 0" 1.0 1.0 0.0 0 0 0 0))

(event Collision|EventHit
  (params (MyComp :type Primitive%20Component%20Object%20Reference) (Other :type Actor%20Object%20Reference) (OtherComp :type Primitive%20Component%20Object%20Reference) (bSelfMoved :type Boolean) (HitLocation :type Vector :default "0, 0, 0") (HitNormal :type Vector :default "0, 0, 0") (NormalImpulse :type Vector :default "0, 0, 0") (Hit :type Hit%20Result%20Structure%20%28by%20ref%29))
  (if (Actor|ActorHasTag Other "Player")
    (bind _asplayer_tp (Utilities|Casting|CastToPlayer_TP Other))
    (Variables|/Game/Character/Main_Character/Player_TP.Player_TP_C|SetHealth _asplayer_tp (- (Variables|/Game/Character/Main_Character/Player_TP.Player_TP_C|GetHealth _asplayer_tp) 1))
    (if (<= (Variables|/Game/Character/Main_Character/Player_TP.Player_TP_C|GetHealth _asplayer_tp) 0)
      (Game|OpenLevel(byName) "Gameover")
      (else
        (Actor|DestroyActor)))
    (else
      (Actor|DestroyActor))))

(fn ConstructionScript)