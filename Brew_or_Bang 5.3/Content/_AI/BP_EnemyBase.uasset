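; BP_EnemyBase is an enemy base Blueprint with health, player chasing and status effects, destroying itself when health runs out.
; ChasePlayer uses AIMoveTo, and on success calls Attack, which only re-issues the chase after a zero delay.
; SlowEnemy temporarily lowers walk speed, then restores a hardcoded value.
; DamageOvertime applies delayed fire damage through a DoN limiter, looping back only after the death check passes.
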(event Custom|SlowEnemy
  (bind _charactermovement (Variables|Character|GetCharacterMovement))
  ;[1 1 1] Slow enemy
  (Variables|/Script/Engine.CharacterMovementComponent|SetMaxWalkSpeed _charactermovement (Variables|Default|GetSlowSpeed))
  (Utilities|FlowControl|Delay (Variables|Default|GetSlowDuration))
  (Variables|/Script/Engine.CharacterMovementComponent|SetMaxWalkSpeed _charactermovement 475.0))

(event Custom|ChasePlayer
  (params (Target :type Pawn%20Object%20Reference))
  (Variables|Default|SetPlayerTarget Target)
  (AI|AIMoveTo self "0, 0, 0" Target 5.0 false
    (:OnSuccess
      (CallFunction|Attack))))

(event Custom|Attack
  (Utilities|FlowControl|Delay 0.0)
  (CallFunction|ChasePlayer (Variables|Default|GetPlayerTarget)))

(event Custom|Death
  (Actor|DestroyActor))

(event Custom|DamageOvertime
  ;[1 1 1] Damage Over Time
  (bind _counter (Utilities|FlowControl|DoN 5 :!label _label)
    (:Exit
      (Utilities|FlowControl|Delay (Variables|Default|GetFireDelay))
      (Development|PrintString (Utilities|String|ToString(Integer) _counter))
      (Variables|Health|SetHealth (- (Variables|Health|GetHealth) (Variables|Default|GetFireDamage)))
      (if (<= (Variables|Health|GetHealth) 0.0)
        (CallFunction|Death)
        (goto _label)))))

(event Game|Damage|EventAnyDamage
  (params (Damage :type Float%20%28single-precision%29) (DamageType :type Damage%20Type%20Object%20Reference) (InstigatedBy :type Controller%20Object%20Reference) (DamageCauser :type Actor%20Object%20Reference))
  (Variables|Health|SetHealth (- (Variables|Health|GetHealth) Damage))
  (if (<= (Variables|Health|GetHealth) 0.0)
    (CallFunction|Death)))

(fn ConstructionScript)