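; BP_save holds the game's persistent data: player health, damage, money, fire and frost unlocks, stage progress and audio volumes.
; LoadSaveGame and SaveGame cast the passed object to the variables class, then run a sequence of small per-field setters to copy values out of or back into the save.
; Saved stage only updates when the incoming stage is equal or higher, so progress never moves backward.
; No disk read or write happens in these graphs.
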(fn LoadSaveGame
  (params (NewParam :type Object%20Object%20Reference))
  (bind _asvariables (Utilities|Casting|CastTovariables NewParam))
  (Utilities|FlowControl|Sequence
    (:then_0
      (|setfire _asvariables))
    (:then_1
      (|setfroze _asvariables))
    (:then_2
      (|setHP _asvariables))
    (:then_3
      (|setMoney _asvariables))
    (:then_4
      (|setMusic _asvariables))
    (:then_5
      (|setDamage _asvariables))
    (:then_6
      (|setSFX _asvariables))
    (:then_7
      (|setStage _asvariables))))

(fn SaveGame
  (params (NewParam :type Object%20Object%20Reference))
  (bind _asvariables (Utilities|Casting|CastTovariables NewParam))
  (Utilities|FlowControl|Sequence
    (:then_0
      (|saveSetFire _asvariables))
    (:then_1
      (|saveSetFroze _asvariables))
    (:then_2
      (|saveSetMaxHP _asvariables))
    (:then_3
      (|saveSetMoney _asvariables))
    (:then_4
      (|saveSetMusic _asvariables))
    (:then_5
      (|saveSetDamage _asvariables))
    (:then_6
      (|saveSetSFX _asvariables))
    (:then_7
      (|saveSetStage _asvariables))))