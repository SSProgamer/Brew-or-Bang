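; Level finish trigger that ends the stage and sends the player to the ShopMenu level.
; On box overlap by any actor, it disables player movement, calls UpdateStage on the variables game instance, then saves.
; Saving only updates an existing "save1" slot through BP_save, never creating one.
; A timeline restarts a camera fade on each update and opens the shop level when finished.
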(event OnComponentBeginOverlap(Box)
  (params (OverlappedComponent :type Primitive%20Component%20Object%20Reference) (OtherActor :type Actor%20Object%20Reference) (OtherComp :type Primitive%20Component%20Object%20Reference) (OtherBodyIndex :type Integer) (bFromSweep :type Boolean) (SweepResult :type Hit%20Result%20Structure%20%28by%20ref%29))
  (Pawn|Components|CharacterMovement|DisableMovement (Variables|/Script/Engine.Character|GetCharacterMovement (Game|GetPlayerCharacter 0)))
  (bind _asvariables (Utilities|Casting|CastTovariables (Game|GetGameInstance)))
  (Default|UpdateStage _asvariables)
  (|saveGame)
  (Utilities|FlowControl|Sequence
    (:then_0
      (Timeline|Timeline_0 Play
        (:Update
          (CameraFades|StartCameraFade :self (Game|GetPlayerCameraManager 0) :FromAlpha 1.0 :Duration 2.0))
        (:Finished
          (Game|OpenLevel(byName) "ShopMenu"))))))

(event EventBeginPlay)

(event Collision|EventActorBeginOverlap
  (params (OtherActor :type Actor%20Object%20Reference)))

(event EventTick
  (params (DeltaSeconds :type Float%20%28single-precision%29)))

(fn ConstructionScript)