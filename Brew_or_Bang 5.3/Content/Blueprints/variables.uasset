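; Shared player-state Blueprint holding stage progress, health, damage, money, bullet unlocks and audio volumes.
; UpdateStage matches the current level name and increments Stage if the stage saved in BP_save slot "save1" is low enough, using four identical load helpers.
; Buy functions check and deduct Money, copied from Player_TP by UpdateMoney, then raise damage or max health, or unlock fire or frost bullets.
; PlayMusic and PlaySfx play 2D sounds at their respective volumes.
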(fn UpdateStage
  (bind _returnvalue (Game|GetCurrentLevelName true))
  (switch string _returnvalue
    (:stage1
      ;[1 1 1] check stage
      (bind _stage (|loadStage))
      (if (< _stage 2)
        (bind _output_get (Variables|Default|Setstage (+ (Variables|Default|Getstage) 1) :!label _label))
        (Development|PrintString (Utilities|String|ToString(Integer) _output_get))))
    (:stage2
      (bind _stage_2 (|loadStage_2))
      (if (< _stage_2 3)
        (goto _label)))
    (:stage3
      (bind _stage_3 (|loadStage_3))
      (if (< _stage_3 4)
        (goto _label)))
    (:stage4
      (bind _stage_4 (|loadStage_2_2))
      (if (< _stage_4 5)
        (goto _label)))))

(fn IncreaseMaxHealth
  (params (number%20to%20increase :type Integer))
  (bind _output_get (Variables|Default|Setmax_health (+ (Variables|Default|Getmax_health) number%20to%20increase)))
  (Development|PrintString (Utilities|String|Append "Max Health:" (Utilities|String|ToString(Integer) _output_get))))

(fn IncreaseHealth
  (params (number%20to%20increase :type Integer))
  (if (> (+ (Variables|Default|Gethealth) number%20to%20increase) (Variables|Default|Getmax_health))
    _
    (else
      (bind _output_get (Variables|Default|Sethealth (+ (Variables|Default|Gethealth) number%20to%20increase)))))
  (Development|PrintString (Utilities|String|Append "Health:" (Utilities|String|ToString(Integer) _output_get) "/" (Utilities|String|ToString(Integer) (Variables|Default|Getmax_health)))))

(fn UpdateMoney
  (bind _asplayer_tp (Utilities|Casting|CastToPlayer_TP (Game|GetPlayerCharacter 0)))
  (Variables|Default|Setmoney (Variables|/Game/Character/Main_Character/Player_TP.Player_TP_C|GetMoney _asplayer_tp)))

(fn IncreasePlayerDamage
  (Variables|Default|Setplayer_damage (+ (Variables|Default|Getplayer_damage) 1.0))
  (Development|PrintString "increase dmg by john"))

(fn UnlockFire
  (Variables|Default|SetfireUnlock true)
  (Development|PrintString "You unlocked fire bullet!"))

(fn UnlockFrost
  (Variables|Default|SetfrozeUnlock true)
  (Development|PrintString "You unlocked froze bullet!"))

(fn BuyFrost
  (params (price :type Integer))
  (if (and (not (Variables|Default|GetfrozeUnlock)) (>= (Variables|Default|Getmoney) price))
    (Variables|Default|Setmoney (- (Variables|Default|Getmoney) price))
    (CallFunction|UnlockFrost)
    (else
      (Development|PrintText "you broke"))))

(fn BuyFire
  (params (price :type Integer))
  (if (and (not (Variables|Default|GetfireUnlock)) (>= (Variables|Default|Getmoney) price))
    (Variables|Default|Setmoney (- (Variables|Default|Getmoney) price))
    (CallFunction|UnlockFire)
    (else
      (Development|PrintText "purchase unsucc"))))

(fn BuyDmg
  (params (price :type Integer))
  (if (>= (Variables|Default|Getmoney) price)
    (Variables|Default|Setmoney (- (Variables|Default|Getmoney) price))
    (CallFunction|IncreasePlayerDamage)
    (else
      (Development|PrintText "purchase unsucc"))))

(fn BuyHP
  (params (price :type Integer))
  (if (>= (Variables|Default|Getmoney) price)
    (Variables|Default|Setmoney (- (Variables|Default|Getmoney) price))
    (CallFunction|IncreaseMaxHealth 2)
    (else
      (Development|PrintText "purchase unsucc"))))

(fn PlayMusic
  (params (music :type Sound%20Base%20Object%20Reference))
  (Audio|PlaySound2D music (Variables|Default|GetmusicVolume) 1.0 0.0 0 0))

(fn PlaySfx
  (params (sound%20Effect :type Sound%20Base%20Object%20Reference))
  (Audio|PlaySound2D sound%20Effect (Variables|Default|GetSFXVolume) 1.0 0.0 0 0))