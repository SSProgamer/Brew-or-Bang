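; BP_EnemyBase is a base enemy Blueprint that takes damage and chases a player target.
; AnyDamage subtracts from Health and calls Death at zero or below, which destroys the actor.
; ChasePlayer stores the target and runs AI MoveTo, calling Attack only on success.
; Attack deals no damage here; it waits on a zero-length Delay and calls ChasePlayer again, forming a chase loop.
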(event Custom|Death
  (Actor|DestroyActor))

(event Custom|ChasePlayer
  (params (Target :type Pawn%20Object%20Reference))
  (Variables|Default|SetPlayerTarget Target)
  (AI|AIMoveTo self "0, 0, 0" Target 5.0 false
    (:OnSuccess
      (CallFunction|Attack))))

(event Custom|Attack
  (Utilities|FlowControl|Delay 0.0)
  (CallFunction|ChasePlayer (Variables|Default|GetPlayerTarget)))

(event EventBeginPlay)

(event Collision|EventActorBeginOverlap
  (params (OtherActor :type Actor%20Object%20Reference)))

(event EventTick
  (params (DeltaSeconds :type Float%20%28single-precision%29)))

(event Game|Damage|EventAnyDamage
  (params (Damage :type Float%20%28single-precision%29) (DamageType :type Damage%20Type%20Object%20Reference) (InstigatedBy :type Controller%20Object%20Reference) (DamageCauser :type Actor%20Object%20Reference))
  (Variables|Health|SetHealth (- (Variables|Health|GetHealth) Damage))
  (if (<= (Variables|Health|GetHealth) 0.0)
    (CallFunction|Death)))

(fn ConstructionScript)